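; BP_XunFeiIAT is a push-to-talk speech recognition actor built on XunFei IAT (dictation) functions.
; On BeginPlay it enables input and the mouse cursor, initializes IAT and adds a WBP_Show widget to the viewport.
; Holding T records and releasing it stops; the OnResult event converts the JSON result to text and displays it in that widget.
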(event EventBeginPlay
  (bind _returnvalue (Game|GetPlayerController 0))
  (Input|EnableInput _returnvalue)
  (Variables|/Script/Engine.PlayerController|SetbShowMouseCursor _returnvalue true)
  (Class|XunFeiIAT|InitXunFeiIAT)
  (bind _returnvalue_2 (UserInterface|CreateWidget "/XunFeiSpeechToText/WBP_Show.WBP_Show_C" _returnvalue))
  (bind _output_get (Variables|Default|SetWBP_Show _returnvalue_2))
  (UserInterface|Viewport|AddtoViewport _output_get 0))

(event EventOnResult
  (params (Result :type String))
  (bind _returnvalue (Class|XunFeiIAT|ConvertJsonResulttoText))
  (bind _wbp_show (Variables|Default|GetWBP_Show)
    (:then
      (Default|ShowResult _wbp_show _returnvalue))
    (:else)))

(event Input|KeyboardEvents|T
  (params (Key :type Key%20Structure :default "None"))
  (:Pressed
    (Class|XunFeiIAT|StartRecord))
  (:Released
    (Class|XunFeiIAT|StopRecord)))

(fn ConstructionScript)